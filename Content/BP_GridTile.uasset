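; BP_GridTile is a single grid tile with a static mesh and a Selector component that marks selection.
; SetOtherColor flags the tile as the other color and swaps its mesh to a black unlit material.
; OnSelection shows or hides the Selector and resets it to the default selector material.
; The construction script only prints the color flag; its branch does nothing.
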(event `SetOtherColor`
  (set `self.IsOtherColor` true)
  (`PrimitiveComponent.SetMaterial` (`self.StaticMesh`) 0 "/Engine/EngineDebugMaterials/BlackUnlitMaterial.BlackUnlitMaterial"))

(event `self.OnSelection`
  (params (isSelected :type Boolean))
  (`SceneComponent.SetHiddenInGame` (`self.Selector`) (not isSelected) false)
  (`PrimitiveComponent.SetMaterial` (`self.Selector`) 0 "/Game/Materials/MI_SelectorDefault.MI_SelectorDefault"))

(fn `UserConstructionScript`
  (bind _isothercolor (`self.IsOtherColor`))
  (`KismetSystemLibrary.PrintString` (`KismetStringLibrary.Conv_BoolToString` _isothercolor))
  (if _isothercolor
    _))