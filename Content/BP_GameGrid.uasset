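; BP_GameGrid is a grid board actor that lays out a checkerboard of tiles for the game.
; Its construction script runs a 2D grid macro sized by depth and width variables, adding a child actor component of the configured square class at each cell center.
; Each child is cast to BP_GridTile, and cells with an odd row-plus-column sum switch to the alternate color.
; The event graph holds no logic.
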(event `self.ReceiveBeginPlay`)

(fn `UserConstructionScript`
  (bind (_current_point _total_points _0_1_phase _poly_center _x_row _y_row) (`/Engine/ArtTools/RenderToTexture/Macros/RenderToTextureMacros.2D Grid Execution Macro` 100.0 (0.0 0.0 0.0) (`self.mNbDepth`) (`self.mNbWidth`))
    (:`Per Poly Execution`
      (bind _returnvalue (`AddComponent|NODE_AddChildActorComponent-0` :`RelativeTransform` (`KismetMathLibrary.Conv_VectorToTransform` _poly_center)))
      (`ChildActorComponent.SetChildActorClass` _returnvalue (`|ConvertAsset` (`self.mSquareActorClass`)))
      (bind _asbp_grid_square (cast `/Game/BP_GridTile` (`ChildActorComponent.ChildActor` _returnvalue)))
      (if (== (mod (+ _x_row _y_row) 2) 1)
        (`/Game/BP_GridTile.SetOtherColor` _asbp_grid_square)))))