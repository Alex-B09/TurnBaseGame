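; Base character Blueprint for tile-based movement, with damage display and teleporting.
; Move calls MoveFromTo for each successive tile pair without waiting; each call restarts a timeline that lerps location between tile character positions and brackets it with MovementStarted and MovementFinished.
; ShowDamage passes a float gameplay attribute to the damage text widget.
; Teleport jumps straight to a tile's position and rotation.
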(event `MoveFromTo`
  (params (From :type "GridTile Object Reference") (To :type "GridTile Object Reference"))
  (bind _returnvalue_location (`KismetMathLibrary.BreakTransform` (`GridTile.GetCharacterPosition` To)))
  (bind _returnvalue_location_2 (`KismetMathLibrary.BreakTransform` (`GridTile.GetCharacterPosition` From)))
  (`self.MovementStarted`)
  (bind (_direction _value) (`Timeline|MoveTimeline` :!via `PlayFromStart`)
    (:`Update`
      (`self.K2_SetActorLocation` (`KismetMathLibrary.VLerp` _returnvalue_location_2 _returnvalue_location _value)))
    (:`Finished`
      (`self.MovementFinished`))))

(event `ShowDamage`
  (bind _asw_dmg_text (cast `/Game/Widgets/W_DmgText` (`WidgetComponent.GetUserWidgetObject` (`self.DmgWidget`))))
  (`/Game/Widgets/W_DmgText.SetDmg` _asw_dmg_text (`.ReturnValue` (`AbilitySystemBlueprintLibrary.GetFloatAttribute` self (struct :`AttributeName` "DamageToApply" :`Attribute` "/Script/TurnBasedGame.CharacterAttributes:DamageToApply")))))

(event `self.Teleport`
  (params (tileToTeleportTo :type "GridTile Object Reference"))
  (bind (_returnvalue_location _returnvalue_rotation) (`KismetMathLibrary.BreakTransform` (`GridTile.GetCharacterPosition` tileToTeleportTo)))
  (`self.K2_TeleportTo` _returnvalue_location _returnvalue_rotation))

(fn `Move`
  (params (currentTile :type "GridTile Object Reference") (tilesToGo :type "Array of GridTile Object Reference (by ref)"))
  (locals (LastTile :type "GridTile Object Reference"))
  (set `local.LastTile` currentTile)
  (for _array_element tilesToGo
    (`self.MoveFromTo` (`local.LastTile`) _array_element)
    (set `local.LastTile` _array_element)))

(fn `UserConstructionScript`)