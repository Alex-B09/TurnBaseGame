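; GA_Movement is a Gameplay Ability that moves the avatar GameCharacter to a tile chosen during activation.
; An async tile-selection task waits for a select or cancel, and a valid tile is passed to the GameplaySubsystem's MoveCharacter.
; The ability ends after moving, on cancel, or after printing an error for an invalid tile, and OnEndAbility ends the stored task.
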(event `self.K2_ActivateAbility`
  (bind (_asynctaskproxy _tile) (`TBG_WaitForTileSelection.WaitForTileSlection` true)
    (:`then`
      (set `self.Wait Task` _asynctaskproxy))
    (:`OnActionSelect`
      (`/Engine/EditorBlueprintResources/StandardMacros.IsValid` _tile
        (:`Is Valid`
          (`GameplaySubsystem.MoveCharacter` (subsystem `GameplaySubsystem`) (cast `GameCharacter` (`self.GetAvatarActorFromActorInfo`) :!pure true) _tile)
          (`self.K2_EndAbility`))
        (:`Is Not Valid`
          (`KismetSystemLibrary.PrintString` "GA_Movement-error")
          (`self.K2_EndAbility`))))
    (:`OnCancel`
      (`self.K2_EndAbility`))))

(event `self.K2_OnEndAbility`
  (params (bWasCancelled :type Boolean))
  (`GameplayTask.EndTask` (`self.Wait Task`)))